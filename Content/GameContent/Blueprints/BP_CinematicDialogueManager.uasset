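; BP_CinematicDialogueManager shows timed on-screen narration for the village of Windrise's intro and the quest-completion outro.
; Shortly after BeginPlay it creates a WB_Dialogue widget and steps through the intro lines, which explain the creature-collecting quest, using hardcoded Delays.
; DialogueFinishTimeline re-adds the same widget to show congratulations, then opens MenuLevel.
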(event `self.ReceiveBeginPlay`
  (`KismetSystemLibrary.Delay` 6.0)
  (bind _returnvalue (`|CreateWidget` "/Game/GameContent/Widgets/WB_Dialogue.WB_Dialogue_C"))
  (bind _output_get (set `self.DialogueWB` _returnvalue))
  (`UserWidget.AddToViewport` _output_get 0)
  (`self.DialogueTimeLine`))

(event `DialogueTimeLine`
  (`/Game/GameContent/Widgets/WB_Dialogue.DialogueText` (`self.DialogueWB`) "This is a small village Windrise")
  (`KismetSystemLibrary.Delay` 3.0)
  (`/Game/GameContent/Widgets/WB_Dialogue.DialogueText` (`self.DialogueWB`) "a beauty full village with temple, houses and water stream")
  (`KismetSystemLibrary.Delay` 6.7)
  (`/Game/GameContent/Widgets/WB_Dialogue.DialogueText` (`self.DialogueWB`) "don't get too lost in it's beauty tho")
  (`KismetSystemLibrary.Delay` 7.0)
  (`/Game/GameContent/Widgets/WB_Dialogue.DialogueText` (`self.DialogueWB`) "your quest here is to collect all the creatures around... ")
  (`KismetSystemLibrary.Delay` 7.8)
  (`/Game/GameContent/Widgets/WB_Dialogue.DialogueText` (`self.DialogueWB`) "and hand them to trader")
  (`KismetSystemLibrary.Delay` 8.0)
  (`/Game/GameContent/Widgets/WB_Dialogue.DialogueText` (`self.DialogueWB`) "")
  (`Widget.RemoveFromParent` (`self.DialogueWB`)))

(event `DialogueFinishTimeline`
  (bind _dialoguewb (`self.DialogueWB`))
  (bind _dialoguewb_2 (`self.DialogueWB`))
  (`UserWidget.AddToViewport` _dialoguewb_2 0)
  (`/Game/GameContent/Widgets/WB_Dialogue.DialogueText` _dialoguewb_2 "Congratulations On Completing all the quest")
  (`KismetSystemLibrary.Delay` 5.0)
  (`/Game/GameContent/Widgets/WB_Dialogue.DialogueText` (`self.DialogueWB`) "See ya on another Quest!!")
  (`KismetSystemLibrary.Delay` 3.6)
  (`/Game/GameContent/Widgets/WB_Dialogue.DialogueText` _dialoguewb "")
  (`Widget.RemoveFromParent` _dialoguewb)
  (`GameplayStatics.OpenLevel` "MenuLevel"))

(fn `UserConstructionScript`)