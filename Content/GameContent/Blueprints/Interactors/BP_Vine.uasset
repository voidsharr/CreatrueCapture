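; BP_Vine is an interactable vine that moves the player to its skeletal mesh's transform when used.
; A box overlap shows and hides its widget, which starts hidden.
; Interaction plays the player widget's Door animation, waits briefly, then reverses it and sets the player's capsule to the mesh transform.
; Gravity toggles for the capsule are present but unconnected, so they never run.
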(event `self.ReceiveBeginPlay`
  (`parent.ReceiveBeginPlay`)
  (`SceneComponent.SetVisibility` (`self.Widget`) false false))

(event `self.Interaction`
  (params (PlayerReference :type "/Game/GameContent/Blueprints/Player/P_Player Object Reference"))
  (bind _playerwidget (`/Game/GameContent/Blueprints/Player/P_Player.PlayerWidget` PlayerReference))
  (bind _door (`/Game/GameContent/Widgets/WB_PlayerMain.door` _playerwidget))
  (`UserWidget.PlayAnimationForward` _playerwidget _door 1.0 false)
  (`KismetSystemLibrary.Delay` 0.8)
  (`UserWidget.PlayAnimationReverse` _playerwidget _door 1.0 false)
  (`SceneComponent.K2_SetWorldTransform` (`Character.CapsuleComponent` PlayerReference) (`SceneComponent.K2_GetComponentToWorld` (`self.SkeletalMesh`)) false false))

(event `self.Box.OnComponentBeginOverlap`
  (params (OverlappedComponent :type "PrimitiveComponent Object Reference") (OtherActor :type "Actor Object Reference") (OtherComp :type "PrimitiveComponent Object Reference") (OtherBodyIndex :type Integer) (bFromSweep :type Boolean) (SweepResult :type "HitResult Structure (by ref)"))
  (`SceneComponent.SetVisibility` (`self.Widget`) true false))

(event `self.Box.OnComponentEndOverlap`
  (params (OverlappedComponent :type "PrimitiveComponent Object Reference") (OtherActor :type "Actor Object Reference") (OtherComp :type "PrimitiveComponent Object Reference") (OtherBodyIndex :type Integer))
  (`SceneComponent.SetVisibility` (`self.Widget`) false false))

(fn `UserConstructionScript`
  (`parent.UserConstructionScript`))