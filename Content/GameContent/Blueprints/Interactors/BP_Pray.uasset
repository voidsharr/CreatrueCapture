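; BP_Pray is an interactor that gives the player a gameplay hint through the dialogue UI.
; On BeginPlay it hides its prompt widget and picks one random entry from its Comment array, so the hint stays the same for that play session.
; Box overlaps toggle the widget's visibility, and the Interaction event sends the chosen text to the player widget under the "Hint" owner.
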(event `self.ReceiveBeginPlay`
  (`parent.ReceiveBeginPlay`)
  (`SceneComponent.SetVisibility` (`self.Widget`) false false)
  (set `self.RandomSelectedHint` (`KismetArrayLibrary.Array_Random` (`self.Comment`))))

(event `/Game/GameContent/Interfaces/BPI_Interact.Interaction`
  (params (PlayerReference :type "/Game/GameContent/Blueprints/Player/P_Player Object Reference"))
  (`/Game/GameContent/Widgets/WB_PlayerMain.SetDialogueText` (`/Game/GameContent/Blueprints/Player/P_Player.PlayerWidget` PlayerReference) "Hint" (`self.RandomSelectedHint`) 2.2 " : "))

(event `self.Box.OnComponentBeginOverlap`
  (params (OverlappedComponent :type "PrimitiveComponent Object Reference") (OtherActor :type "Actor Object Reference") (OtherComp :type "PrimitiveComponent Object Reference") (OtherBodyIndex :type Integer) (bFromSweep :type Boolean) (SweepResult :type "HitResult Structure (by ref)"))
  (`SceneComponent.SetVisibility` (`self.Widget`) true false))

(event `self.Box.OnComponentEndOverlap`
  (params (OverlappedComponent :type "PrimitiveComponent Object Reference") (OtherActor :type "Actor Object Reference") (OtherComp :type "PrimitiveComponent Object Reference") (OtherBodyIndex :type Integer))
  (`SceneComponent.SetVisibility` (`self.Widget`) false false))

(fn `UserConstructionScript`
  (`parent.UserConstructionScript`))