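; BP_Creature is an interactable creature pickup whose ECreatureSelf type selects its skeletal mesh at construction and its looping idle or dizzy animation at BeginPlay.
; On Interaction, a player already holding something gets a random refusal line.
; Otherwise the player is locked, marked as holding and tagged with the type.
; The SenseAnimation macro then switches animation and continues to pickup dialogue, a short delay, movement release and the creature's destruction.
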(event `self.ReceiveBeginPlay`
  (`parent.ReceiveBeginPlay`)
  (switch `/Game/GameContent/Blueprints/E_Creature` (`self.E_CreatureSelf`)
    (:`NewEnumerator0`
      (`SkeletalMeshComponent.PlayAnimation` (`self.SkeletalMesh`) null false))
    (:`NewEnumerator1`
      (`SkeletalMeshComponent.PlayAnimation` (`self.SkeletalMesh`) "/Game/MonsterForSurvivalGame/Animation/PBR/Cactus/Cactus_Dizzy_ANIM.Cactus_Dizzy_ANIM" true))
    (:`NewEnumerator2`
      (`SkeletalMeshComponent.PlayAnimation` (`self.SkeletalMesh`) "/Game/MonsterForSurvivalGame/Animation/PBR/Mushroom/SmileVersion/Mushroom_DizzySmile_ANIM.Mushroom_DizzySmile_ANIM" true))
    (:`NewEnumerator3`
      (`SkeletalMeshComponent.PlayAnimation` (`self.SkeletalMesh`) "/Game/MonsterForSurvivalGame/Animation/PBR/TurtleShell/TurtleShell_Dizzy_ANIM.TurtleShell_Dizzy_ANIM" true))
    (:`NewEnumerator4`
      (`SkeletalMeshComponent.PlayAnimation` (`self.SkeletalMesh`) "/Game/MonsterForSurvivalGame/Animation/PBR/Swarm08/Swarm08_Idle_Anim.Swarm08_Idle_Anim" true))
    (:`NewEnumerator5`
      (`SkeletalMeshComponent.PlayAnimation` (`self.SkeletalMesh`) "/Game/MonsterForSurvivalGame/Animation/PBR/Swarm09/Swarm09_Idle_Anim.Swarm09_Idle_Anim" true))
    (:`NewEnumerator6`
      (`SkeletalMeshComponent.PlayAnimation` (`self.SkeletalMesh`) "/Game/MonsterForSurvivalGame/Animation/PBR/Slime/Slime_Dizzy_ANIM.Slime_Dizzy_ANIM" true))
    (:`NewEnumerator7`
      (`SkeletalMeshComponent.PlayAnimation` (`self.SkeletalMesh`) "/Game/MonsterForSurvivalGame/Animation/PBR/ChestMonster/ChestMonster_Dizzy_ANIM.ChestMonster_Dizzy_ANIM" true))))

(event `/Game/GameContent/Interfaces/BPI_Interact.Interaction`
  (params (PlayerReference :type "/Game/GameContent/Blueprints/Player/P_Player Object Reference"))
  (bind _skeletalmesh (`self.SkeletalMesh`))
  (bind _skeletalmesh_2 (`self.SkeletalMesh`))
  (bind _e_creatureself (`self.E_CreatureSelf`))
  (if (`/Game/GameContent/Blueprints/Player/P_Player.Holding?` PlayerReference)
    (if (`self.Not on Text`)
      (`/Game/GameContent/Widgets/WB_PlayerMain.SetDialogueText` (`/Game/GameContent/Blueprints/Player/P_Player.PlayerWidget` PlayerReference) (`|GetEnumeratorNameAsString` (`self.E_CreatureSelf`)) (`KismetArrayLibrary.Array_Random` (`self.UnableDialogue`)) 2.2 " : ")
      (`KismetSystemLibrary.Delay` 2.5)
      (set `self.Not on Text` true))
    (else
      (set `/Game/GameContent/Blueprints/Player/P_Player.bDisableMov` true PlayerReference)
      (set `/Game/GameContent/Blueprints/Player/P_Player.Holding?` true PlayerReference)
      (`KismetArrayLibrary.Array_AddUnique` (`/Game/GameContent/Blueprints/Player/P_Player.E_CreaturesTag` PlayerReference) (`self.E_CreatureSelf`))
      (switch `/Game/GameContent/Blueprints/E_Creature` (`self.E_CreatureSelf`)
        (:`NewEnumerator0`
          (`SkeletalMeshComponent.PlayAnimation` _skeletalmesh null false))
        (:`NewEnumerator1`
          (`SkeletalMeshComponent.PlayAnimation` _skeletalmesh "/Game/MonsterForSurvivalGame/Animation/PBR/Cactus/Cactus_SenseSomethingMaint_ANIM.Cactus_SenseSomethingMaint_ANIM" true)
          (`/Game/GameContent/Widgets/WB_PlayerMain.SetDialogueText` (`/Game/GameContent/Blueprints/Player/P_Player.PlayerWidget` PlayerReference) (`|GetEnumeratorNameAsString` _e_creatureself) (`BlueprintMapLibrary.Map_Find` (`self.DialogueOnPick`) _e_creatureself) 2.2 " : " :!label _label)
          (`KismetSystemLibrary.Delay` 1.8)
          (set `/Game/GameContent/Blueprints/Player/P_Player.bDisableMov` false PlayerReference)
          (`self.K2_DestroyActor`))
        (:`NewEnumerator2`
          (`SkeletalMeshComponent.PlayAnimation` _skeletalmesh "/Game/MonsterForSurvivalGame/Animation/PBR/Mushroom/SmileVersion/Mushroom_SenseSomethingMaintainSmile_ANIM.Mushroom_SenseSomethingMaintainSmile_ANIM" true)
          (goto _label))
        (:`NewEnumerator3`
          (`SkeletalMeshComponent.PlayAnimation` _skeletalmesh "/Game/MonsterForSurvivalGame/Animation/PBR/TurtleShell/TurtleShell_SenseSomethingRT_ANIM.TurtleShell_SenseSomethingRT_ANIM" true)
          (goto _label))
        (:`NewEnumerator4`
          (`SkeletalMeshComponent.PlayAnimation` _skeletalmesh "/Game/MonsterForSurvivalGame/Animation/PBR/Swarm08/Swarm08_MoveFWD_Anim.Swarm08_MoveFWD_Anim" true)
          (goto _label))
        (:`NewEnumerator5`
          (`SkeletalMeshComponent.PlayAnimation` _skeletalmesh_2 "/Game/MonsterForSurvivalGame/Animation/PBR/Swarm09/Swarm09_MoveFWD_Anim.Swarm09_MoveFWD_Anim" true)
          (goto _label))
        (:`NewEnumerator6`
          (`SkeletalMeshComponent.PlayAnimation` _skeletalmesh_2 "/Game/MonsterForSurvivalGame/Animation/PBR/Slime/Slime_SenseSomethingRoutine_ANIM.Slime_SenseSomethingRoutine_ANIM" true)
          (goto _label))
        (:`NewEnumerator7`
          (`SkeletalMeshComponent.PlayAnimation` _skeletalmesh_2 "/Game/MonsterForSurvivalGame/Animation/PBR/ChestMonster/ChestMonster_SenseSomethingRPT_ANIM.ChestMonster_SenseSomethingRPT_ANIM" true)
          (goto _label))))))

(fn `UserConstructionScript`
  (`parent.UserConstructionScript`)
  (switch `/Game/GameContent/Blueprints/E_Creature` (`self.E_CreatureSelf`)
    (:`NewEnumerator0`
      (`SkeletalMeshComponent.SetSkeletalMeshAsset` (`self.SkeletalMesh`) null))
    (:`NewEnumerator1`
      (`SkeletalMeshComponent.SetSkeletalMeshAsset` (`self.SkeletalMesh`) "/Game/MonsterForSurvivalGame/Mesh/PBR/Cactus_SK.Cactus_SK"))
    (:`NewEnumerator2`
      (`SkeletalMeshComponent.SetSkeletalMeshAsset` (`self.SkeletalMesh`) "/Game/MonsterForSurvivalGame/Mesh/PBR/Mushroom_SK.Mushroom_SK"))
    (:`NewEnumerator3`
      (`SkeletalMeshComponent.SetSkeletalMeshAsset` (`self.SkeletalMesh`) "/Game/MonsterForSurvivalGame/Mesh/PBR/TurtleShell_SK.TurtleShell_SK"))
    (:`NewEnumerator4`
      (`SkeletalMeshComponent.SetSkeletalMeshAsset` (`self.SkeletalMesh`) "/Game/MonsterForSurvivalGame/Mesh/PBR/Swarm08_SK.Swarm08_SK"))
    (:`NewEnumerator5`
      (`SkeletalMeshComponent.SetSkeletalMeshAsset` (`self.SkeletalMesh`) "/Game/MonsterForSurvivalGame/Mesh/PBR/Swarm09_SK.Swarm09_SK"))
    (:`NewEnumerator6`
      (`SkeletalMeshComponent.SetSkeletalMeshAsset` (`self.SkeletalMesh`) "/Game/MonsterForSurvivalGame/Mesh/PBR/Slime_SK.Slime_SK"))
    (:`NewEnumerator7`
      (`SkeletalMeshComponent.SetSkeletalMeshAsset` (`self.SkeletalMesh`) "/Game/MonsterForSurvivalGame/Mesh/PBR/ChestMonster_SK.ChestMonster_SK"))))