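; MedKeeper is an interactable NPC that receives the creatures a player carries and tracks progress toward finishing the quest.
; With none carried it shows a throttled random line; otherwise it moves the first creature tag into its reached list and briefly freezes the player.
; It celebrates with animation and dialogue, switching a victory mesh to the matching creature.
; Once the list reaches the NumOfCreatures index, it completes the quest, fades out and disables input.
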(event `/Game/GameContent/Interfaces/BPI_Interact.Interaction`
  (params (PlayerReference :type "/Game/GameContent/Blueprints/Player/P_Player Object Reference"))
  (bind _victorymesh (`self.VictoryMesh`))
  (bind _victorymesh_2 (`self.VictoryMesh`))
  (bind _e_creaturestag (`/Game/GameContent/Blueprints/Player/P_Player.E_CreaturesTag` PlayerReference))
  (bind _e_creaturestag_2 (`/Game/GameContent/Blueprints/Player/P_Player.E_CreaturesTag` PlayerReference))
  (bind _output (`|GetArrayItem` _e_creaturestag))
  (set `self.E Creatures Tag` _e_creaturestag_2)
  (if (`KismetArrayLibrary.Array_IsEmpty` _e_creaturestag_2)
    (if (`self.Not on Text`)
      (set `self.Not on Text` false)
      (`/Game/GameContent/Widgets/WB_PlayerMain.SetDialogueText` (`/Game/GameContent/Blueprints/Player/P_Player.PlayerWidget` PlayerReference) "MedKeeper" (`KismetArrayLibrary.Array_Random` (`self.EmptyDialogues`)) 2.2 " : ")
      (`KismetSystemLibrary.Delay` 2.5)
      (set `self.Not on Text` true))
    (else
      (set `/Game/GameContent/Blueprints/Player/P_Player.Holding?` false PlayerReference)
      (set `/Game/GameContent/Blueprints/Player/P_Player.bDisableMov` true PlayerReference)
      (`KismetArrayLibrary.Array_AddUnique` (`self.E_CreatureReached`) _output)
      (`KismetArrayLibrary.Array_RemoveItem` _e_creaturestag _output)
      (`SkeletalMeshComponent.PlayAnimation` (`self.MSkeletalMesh`) "/Game/BattleWizardPolyart/Animations/VictoryStartAnim.VictoryStartAnim" false)
      (`|ExecutionSequence`
        (:`then_0`
          (`KismetSystemLibrary.Delay` 3.0)
          (`SkeletalMeshComponent.PlayAnimation` (`self.MSkeletalMesh`) "/Game/BattleWizardPolyart/Animations/VictoryMaintainAnim.VictoryMaintainAnim" true)
          (set `/Game/GameContent/Blueprints/Player/P_Player.bDisableMov` false PlayerReference))
        (:`then_1`
          (`|ExecutionSequence`
            (:`then_0`
              (`/Game/GameContent/Blueprints/Player/P_Player.HideMeshAsset` PlayerReference)
              (if (`KismetArrayLibrary.Array_IsValidIndex` (`self.E_CreatureReached`) (`self.NumOfCreatures`))
                (set `self.QuestCompleted` true)
                (`/Game/GameContent/Widgets/WB_PlayerMain.FinalFade` (`/Game/GameContent/Blueprints/Player/P_Player.PlayerWidget` PlayerReference))
                (`self.DisableInput` PlayerReference (`GameplayStatics.GetPlayerController` 0))
                (`/Game/GameContent/Blueprints/BP_CinematicDialogueManager.DialogueFinishTimeline` (`self.DialogueManager`))))
            (:`then_1`
              (switch `/Game/GameContent/Blueprints/E_Creature` (`|GetArrayItem` (`self.E Creatures Tag`))
                (:`NewEnumerator0`
                  (`self.SetMeshAnimAsset` _victorymesh_2))
                (:`NewEnumerator1`
                  (`self.SetMeshAnimAsset` _victorymesh_2 "/Game/MonsterForSurvivalGame/Mesh/PBR/Cactus_SK.Cactus_SK" "/Game/MonsterForSurvivalGame/Animation/PBR/Cactus/Cactus_Victory_ANIM.Cactus_Victory_ANIM" true))
                (:`NewEnumerator2`
                  (`self.SetMeshAnimAsset` _victorymesh_2 "/Game/MonsterForSurvivalGame/Mesh/PBR/Mushroom_SK.Mushroom_SK" "/Game/MonsterForSurvivalGame/Animation/PBR/Mushroom/SmileVersion/Mushroom_VictorySmile_ANIM.Mushroom_VictorySmile_ANIM" true))
                (:`NewEnumerator3`
                  (`self.SetMeshAnimAsset` _victorymesh_2 "/Game/MonsterForSurvivalGame/Mesh/PBR/TurtleShell_SK.TurtleShell_SK" "/Game/MonsterForSurvivalGame/Animation/PBR/TurtleShell/TurtleShell_Victory_ANIM.TurtleShell_Victory_ANIM" true))
                (:`NewEnumerator4`
                  (`self.SetMeshAnimAsset` _victorymesh_2 "/Game/MonsterForSurvivalGame/Mesh/PBR/Swarm08_SK.Swarm08_SK" "/Game/MonsterForSurvivalGame/Animation/PBR/Swarm08/Swarm08_Idle_Anim.Swarm08_Idle_Anim" true))
                (:`NewEnumerator5`
                  (`self.SetMeshAnimAsset` _victorymesh "/Game/MonsterForSurvivalGame/Mesh/PBR/Swarm09_SK.Swarm09_SK" "/Game/MonsterForSurvivalGame/Animation/PBR/Swarm08/Swarm08_Idle_Anim.Swarm08_Idle_Anim" true))
                (:`NewEnumerator6`
                  (`self.SetMeshAnimAsset` _victorymesh "/Game/MonsterForSurvivalGame/Mesh/PBR/Slime_SK.Slime_SK" "/Game/MonsterForSurvivalGame/Animation/PBR/Slime/Slime_Victory_ANIM.Slime_Victory_ANIM" true))
                (:`NewEnumerator7`
                  (`self.SetMeshAnimAsset` _victorymesh "/Game/MonsterForSurvivalGame/Mesh/PBR/ChestMonster_SK.ChestMonster_SK" "/Game/MonsterForSurvivalGame/Animation/PBR/ChestMonster/ChestMonster_Victory_ANIM.ChestMonster_Victory_ANIM" true)))
              (`KismetSystemLibrary.Delay` 3.0)
              (`self.SetMeshAnimAsset` (`self.VictoryMesh`)))))
        (:`then_2`
          (`/Game/GameContent/Widgets/WB_PlayerMain.SetDialogueText` (`/Game/GameContent/Blueprints/Player/P_Player.PlayerWidget` PlayerReference) "MedKeeper" (`KismetArrayLibrary.Array_Random` (`self.CompleteDialogue`)) 2.2 " : "))))))

(fn `SetMeshAnimAsset`
  (params (Target :type "SkeletalMeshComponent Object Reference") (NewMesh :type "SkeletalMesh Object Reference") (NewAnimToPlay :type "AnimationAsset Object Reference") (bLooping :type Boolean))
  (`SkeletalMeshComponent.SetSkeletalMeshAsset` Target NewMesh)
  (`SkeletalMeshComponent.PlayAnimation` Target NewAnimToPlay bLooping))

(fn `UserConstructionScript`)